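; Base character for a basketball game, handling movement, dribble moves, drive-ins, shooting and defense.
; Input plays skill montages gated on ball possession and attack state, and releasing shoot launches the BP_Ball found at BeginPlay toward the basket.
; Tick computes distance, facing dots and yaw to a target, smoothly turning toward it while IsDefense, which move input sets.
; Helper functions relay ball motion and chain drive-ins; target-relative defense movement is unwired.
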(event `self.ReceiveBeginPlay`
  (`self.InitializeCharacterBase`) ; 변수 초기화
  (bind _outactors (`GameplayStatics.GetAllActorsOfClass` "/Game/Basketball/Blueprints/BP_Ball.BP_Ball_C"))
  (bind _output_get (set `self.CurrentBall` (`|GetArrayItem` _outactors)))
  (set `/Game/Basketball/Blueprints/BP_Ball.OwnerCharacter` self _output_get)
  (set `self.bHasBall` true))

(event `self.ReceiveTick`
  (params (DeltaSeconds :type "Float (single-precision)"))
  (`self.UpdateMovementData`)
  (`self.UpdateTargetRelation`)
  (`self.UpdateDefenseRotation` DeltaSeconds))

(event `EnhancedInput|/Game/Blueprint/Input/Action/IA_Crossover`
  (params (ActionValue :type Boolean) (ElapsedSeconds :type "Float (double-precision)") (TriggeredSeconds :type "Float (double-precision)") (InputAction :type "InputAction Object Reference" :default "/Game/Blueprint/Input/Action/IA_Crossover.IA_Crossover"))
  ; 드리블 모션
  (:`Triggered`
    (`self.StartSkillDribble` "NewEnumerator2" "/Game/Blueprint/Anime/AM_Crossover.AM_Crossover")))

(event `EnhancedInput|/Game/Blueprint/Input/Action/IA_BetweenLeg`
  (params (ActionValue :type Boolean) (ElapsedSeconds :type "Float (double-precision)") (TriggeredSeconds :type "Float (double-precision)") (InputAction :type "InputAction Object Reference" :default "/Game/Blueprint/Input/Action/IA_BetweenLeg.IA_BetweenLeg"))
  ; 드리블 모션
  (:`Triggered`
    (`self.StartSkillDribble` "NewEnumerator3" "/Game/Blueprint/Anime/AM_BetweenLeg.AM_BetweenLeg")))

(event `EnhancedInput|/Game/Blueprint/Input/Action/IA_DriveInL`
  (params (ActionValue :type Boolean) (ElapsedSeconds :type "Float (double-precision)") (TriggeredSeconds :type "Float (double-precision)") (InputAction :type "InputAction Object Reference" :default "/Game/Blueprint/Input/Action/IA_DriveInL.IA_DriveInL"))
  ; 돌파 처리
  (:`Triggered`
    (if (`self.bHasBall`)
      (set `self.QueuedDirection` "NewEnumerator1")
      (`self.StartSkillDribble` "NewEnumerator4" "/Game/Blueprint/Anime/AM_DriveInL.AM_DriveInL"))))

(event `EnhancedInput|/Game/Blueprint/Input/Action/IA_DriveInR`
  (params (ActionValue :type Boolean) (ElapsedSeconds :type "Float (double-precision)") (TriggeredSeconds :type "Float (double-precision)") (InputAction :type "InputAction Object Reference" :default "/Game/Blueprint/Input/Action/IA_DriveInR.IA_DriveInR"))
  ; 돌파 처리
  (:`Triggered`
    (if (`self.bHasBall`)
      (set `self.QueuedDirection` "NewEnumerator2")
      (`self.StartSkillDribble` "NewEnumerator5" "/Game/Blueprint/Anime/AM_DriveInR.AM_DriveInR"))))

(event `EnhancedInput|/Game/Input/Actions/IA_Move`
  (params (ActionValue :type "Vector2D Structure") (ElapsedSeconds :type "Float (double-precision)") (TriggeredSeconds :type "Float (double-precision)") (InputAction :type "InputAction Object Reference" :default "/Game/Input/Actions/IA_Move.IA_Move"))
  (:`Triggered`
    ; 이동 처리, 베이스는 삭제하고 캐릭터에만 남길 예정
    (`self.SetMoveInput` ActionValue_X ActionValue_Y)
    (set `self.bIsDefense` true)
    (`self.AddMovementInput` (`KismetMathLibrary.GetForwardVector` (`self.GetControlRotation`)) ActionValue_X)
    (`self.AddMovementInput` (`KismetMathLibrary.GetRightVector` (`self.GetControlRotation`)) ActionValue_Y))
  (:`Completed`
    (set `self.CurrentDribbleType` "NewEnumerator0")
    (`self.SetMoveInput` 0.0)))

(event `EnhancedInput|/Game/Blueprint/Input/Action/IA_Shoot`
  (params (ActionValue :type Boolean) (ElapsedSeconds :type "Float (double-precision)") (TriggeredSeconds :type "Float (double-precision)") (InputAction :type "InputAction Object Reference" :default "/Game/Blueprint/Input/Action/IA_Shoot.IA_Shoot"))
  (bind _currentball (`self.CurrentBall`))
  (:`Started`
    (set `self.PlayerAttackState` "NewEnumerator7"))
  (:`Completed`
    (`/Engine/EditorBlueprintResources/StandardMacros.IsValid` _currentball
      (:`Is Valid`
        (bind _returnvalue (`GameplayStatics.GetActorOfClass` "/Game/Basketball/Blueprints/BP_Basket.BP_Basket_C"))
        (`/Game/Basketball/Blueprints/BP_Ball.LaunchToTarget` _currentball (`SceneComponent.K2_GetComponentLocation` (`/Game/Basketball/Blueprints/BP_Basket.ShotTarget` _returnvalue)))))))

(fn `ClearTargetActor`
  (set `self.TargetActor` null)
  (set `self.bHasTarget` false)
  (set `self.DistanceToTarget` 0.0)
  (set `self.FrontDot` 0.0)
  (set `self.RightDot` 0.0)
  (set `self.YawDeltaToTarget` 0.0))

(fn `EnterDefense`
  (set `self.bIsDefense` true)
  (set `self.MainState` "NewEnumerator1"))

(fn `ExitDefense`
  (set `self.bIsDefense` false)
  (set `self.MainState` "NewEnumerator0")
  (set `self.DefenseReactionState` "NewEnumerator0"))

(fn `InitializeCharacterBase`
  (set `self.MainState` "NewEnumerator0")
  (set `self.bIsDefense` false)
  (set `self.bHasTarget` false)
  (set `self.MoveInputX` 0.0)
  (set `self.MoveInputY` 0.0))

(fn `NewFunction`)

(fn `OnBallCatch`
  (`/Engine/EditorBlueprintResources/StandardMacros.IsValid` (`self.CurrentBall`)
    (:`Is Valid`
      (`/Game/Basketball/Blueprints/BP_Ball.SetAttached` (`self.CurrentBall`)))))

(fn `OnBallStartDown`
  (`/Engine/EditorBlueprintResources/StandardMacros.IsValid` (`self.CurrentBall`)
    (:`Is Valid`
      (`/Game/Basketball/Blueprints/BP_Ball.StartMoveDown` (`self.CurrentBall`)))))

(fn `OnBallStartUp`
  (`/Engine/EditorBlueprintResources/StandardMacros.IsValid` (`self.CurrentBall`)
    (:`Is Valid`
      (`/Game/Basketball/Blueprints/BP_Ball.StartMoveUp` (`self.CurrentBall`)))))

(fn `PerformDefenseMovement`
  (bind _returnvalue (`KismetMathLibrary.FindLookAtRotation` (`self.K2_GetActorLocation`) (`self.K2_GetActorLocation` (`self.TargetActor`))))
  (if (`self.bIsDefense`)
    (`/Engine/EditorBlueprintResources/StandardMacros.IsValid` (`self.TargetActor`)
      (:`Is Valid`
        (`self.AddMovementInput` (`KismetMathLibrary.GetForwardVector` _returnvalue) (`self.MoveInputY`))
        (`self.AddMovementInput` (`KismetMathLibrary.GetRightVector` _returnvalue) (`self.MoveInputX`))))))

(fn `SetMoveInput`
  (params (NewMoveInputX :type "Float (double-precision)") (NewMoveInputY :type "Float (double-precision)"))
  (set `self.MoveInputX` NewMoveInputX)
  (set `self.MoveInputY` NewMoveInputY))

(fn `SetTargetActor`
  (params (NewTargetactor :type "Actor Object Reference"))
  (bind _output_get (set `self.TargetActor` NewTargetactor))
  (`/Engine/EditorBlueprintResources/StandardMacros.IsValid` _output_get
    (:`Is Valid`
      (set `self.bHasTarget` true))
    (:`Is Not Valid`
      (set `self.bHasTarget` false))))

(fn `StartDribble`
  (set `self.CurrentAttackAction` "NewEnumerator1")
  (set `self.bCanChainDriveIn` false)
  (set `self.QueuedDirection` "NewEnumerator0"))

(fn `StartDriveIn`
  (if (and (`self.bHasBall`) (`self.bCanChainDriveIn`))
    (set `self.bCanChainDriveIn` false)
    (switch `/Game/Blueprint/EDriveDirection` (`self.QueuedDirection`)
      (:`NewEnumerator1`
        (`self.StopAnimMontage` null)
        (set `self.CurrentAttackAction` "NewEnumerator4")
        (set `self.QueuedDirection` "NewEnumerator0")
        (`self.PlayAnimMontage` "/Game/Blueprint/Anime/AM_DriveInL.AM_DriveInL"))
      (:`NewEnumerator2`
        (`self.StopAnimMontage` null)
        (set `self.CurrentAttackAction` "NewEnumerator5")
        (set `self.QueuedDirection` "NewEnumerator0")
        (`self.PlayAnimMontage` "/Game/Blueprint/Anime/AM_DriveInR.AM_DriveInR")))))

(fn `StartSkillDribble`
  (params (NewAction :type "/Game/Blueprint/EAttackAction Enum" :default "NewEnumerator0") (MonTage :type "AnimMontage Object Reference"))
  (if (and (`self.bHasBall`) (`|EnumEquality` "NewEnumerator1" (`self.CurrentAttackAction`)))
    (set `self.CurrentAttackAction` NewAction)
    (set `self.bCanChainDriveIn` false)
    (set `self.QueuedDirection` "NewEnumerator0")
    (`self.PlayAnimMontage` MonTage)))

(fn `StopDribble`
  (set `self.bIsDribbling` false)
  (set `self.bIsSkillDribblingPlaying` false)
  (set `self.CurrentAttackAction` "NewEnumerator0"))

(fn `UpdateDefenseRotation`
  (params (DeltaTime :type "Float (double-precision)"))
  (bind (_returnvalue_roll _returnvalue_pitch _returnvalue_yaw) (`KismetMathLibrary.BreakRotator` (`KismetMathLibrary.FindLookAtRotation` (`self.K2_GetActorLocation`) (`self.K2_GetActorLocation` (`self.TargetActor`)))))
  (if (`self.bIsDefense`)
    (`/Engine/EditorBlueprintResources/StandardMacros.IsValid` (`self.TargetActor`)
      (:`Is Valid`
        (`self.K2_SetActorRotation` (`KismetMathLibrary.RInterpTo` (`self.K2_GetActorRotation`) (`KismetMathLibrary.MakeRotator` 0.0 0.0 _returnvalue_yaw) DeltaTime (`self.DefenseRotationInterpSpeed`)))))))

(fn `UpdateMovementData`
  (set `self.CurrentSpeed` (`KismetMathLibrary.VSize` (`self.GetVelocity`))))

(fn `UpdateTargetRelation`
  (bind _returnvalue (- (`self.K2_GetActorLocation` (`self.TargetActor`)) (`self.K2_GetActorLocation`)))
  (bind (_returnvalue_roll _returnvalue_pitch _returnvalue_yaw) (`KismetMathLibrary.BreakRotator` (`KismetMathLibrary.NormalizedDeltaRotator` (`KismetMathLibrary.FindLookAtRotation` (`self.K2_GetActorLocation`) (`self.K2_GetActorLocation` (`self.TargetActor`))) (`self.K2_GetActorRotation`))))
  (`/Engine/EditorBlueprintResources/StandardMacros.IsValid` (`self.TargetActor`) ; 유효성  확인
    (:`Is Valid`
      (set `self.DistanceToTarget` (`KismetMathLibrary.VSize` _returnvalue))
      ; 앞뒤 계산
      ; FrontDot = Dot(MyForward, ToTargetNormalized)
      ; RightDot = Dot(MyRight, ToTargetNormalized)
      (set `self.FrontDot` (`KismetMathLibrary.Dot_VectorVector` (`self.GetActorForwardVector`) (`KismetMathLibrary.Normal` _returnvalue)))
      (set `self.RightDot` (`KismetMathLibrary.Dot_VectorVector` (`self.GetActorRightVector`) (`KismetMathLibrary.Normal` _returnvalue)))
      ; 타겟을 보기 위해서 얼마나 회전해야 하는지 계산
      (set `self.YawDeltaToTarget` _returnvalue_yaw))
    (:`Is Not Valid`
      (set `self.bHasTarget` false))))

(fn `UserConstructionScript`)