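; Player character for a basketball game, driven by Enhanced Input and a StateBP state set from ball possession at BeginPlay.
; Move, run and layup inputs handle movement, sprint speed and state changes, while C enters Defense.
; In Defense, movement follows actor axes after rotation from DefenseTarget's location vector, though that target's lookup is disconnected.
; Key 1 starts upward movement on the BP_Ball found at BeginPlay.
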(event `Key|One`
  (params (Key :type "Key Structure"))
  (:`Pressed`
    (`/Game/Basketball_template/Blueprints/BP_Ball.StartMoveUp` (`self.CurrentBall`))))

(event `self.ReceiveBeginPlay`
  (`self.UpdatePlayerState`)
  (bind _returnvalue (`GameplayStatics.GetActorOfClass` "/Game/Basketball_template/Blueprints/BP_Ball.BP_Ball_C"))
  (set `self.CurrentBall` _returnvalue))

(event `EnhancedInput|/Game/Input/Actions/IA_Move`
  (params (ActionValue :type "Vector2D Structure") (ElapsedSeconds :type "Float (double-precision)") (TriggeredSeconds :type "Float (double-precision)") (InputAction :type "InputAction Object Reference" :default "/Game/Input/Actions/IA_Move.IA_Move"))
  (bind (_returnvalue_roll _returnvalue_pitch _returnvalue_yaw) (`KismetMathLibrary.BreakRotator` (`self.GetControlRotation`)))
  (bind (_returnvalue_roll_2 _returnvalue_pitch_2 _returnvalue_yaw_2) (`KismetMathLibrary.BreakRotator` (`self.GetControlRotation`)))
  (:`Triggered`
    ; 캐릭터 이동
    (`self.AddMovementInput` (`KismetMathLibrary.GetRightVector` (`KismetMathLibrary.MakeRotator` _returnvalue_roll 0.0 _returnvalue_yaw)) ActionValue_Y)
    (`self.AddMovementInput` (`KismetMathLibrary.GetForwardVector` (`KismetMathLibrary.MakeRotator` 0.0 0.0 _returnvalue_yaw_2)) ActionValue_X)))

(event `EnhancedInput|/Game/Blueprint/Input/Action/IA_Run`
  (params (ActionValue :type Boolean) (ElapsedSeconds :type "Float (double-precision)") (TriggeredSeconds :type "Float (double-precision)") (InputAction :type "InputAction Object Reference" :default "/Game/Blueprint/Input/Action/IA_Run.IA_Run"))
  ; 캐릭터 달리기
  (:`Triggered`
    (set `self.State_BP` "NewEnumerator1")
    (`self.Sprint`))
  (:`Completed`
    (set `self.State_BP` "NewEnumerator0")
    (`self.StopSprint`)))

(event `Key|C`
  (params (Key :type "Key Structure"))
  (:`Pressed`
    (set `self.State_BP` "NewEnumerator6")))

(event `EnhancedInput|/Game/Blueprint/Input/Action/IA_Layup`
  (params (ActionValue :type Boolean) (ElapsedSeconds :type "Float (double-precision)") (TriggeredSeconds :type "Float (double-precision)") (InputAction :type "InputAction Object Reference" :default "/Game/Blueprint/Input/Action/IA_Layup.IA_Layup"))
  ; 레이업
  (:`Triggered`
    (set `self.State_BP` "NewEnumerator4"))
  (:`Completed`
    (set `self.State_BP` "NewEnumerator0")))

(event `EnhancedInput|/Game/Blueprint/Input/Action/IA_DefenseMove`
  (params (ActionValue :type "Vector2D Structure") (ElapsedSeconds :type "Float (double-precision)") (TriggeredSeconds :type "Float (double-precision)") (InputAction :type "InputAction Object Reference" :default "/Game/Blueprint/Input/Action/IA_DefenseMove.IA_DefenseMove"))
  (:`Triggered`
    (bind _output_get (set `self.DefeseHorizontal` ActionValue_Y))
    (bind _output_get_2 (set `self.FollowHorizontal` ActionValue_X))
    (switch `/Game/Blueprint/EPlayerState` (`self.State_BP`) :!label _label
      (:`NewEnumerator6`
        (`/Engine/EditorBlueprintResources/StandardMacros.IsValid` (`self.DefenseTarget`)
          (:`Is Valid`
            (`self.K2_SetActorRotation` (`KismetMathLibrary.Conv_VectorToRotator` (`self.K2_GetActorLocation` (`self.DefenseTarget`))))
            (`self.AddMovementInput` (`KismetMathLibrary.GetRightVector` (`self.K2_GetActorRotation`)) _output_get)
            (`self.AddMovementInput` (`KismetMathLibrary.GetForwardVector` (`self.K2_GetActorRotation`)) _output_get_2))))))
  (:`Completed`
    (set `self.DefeseHorizontal` 0.0)
    (set `self.FollowHorizontal` 0.0)
    (goto _label)))

(fn `Sprint`
  (set `CharacterMovementComponent.MaxWalkSpeed` (`self.SprintSpeed`) (`self.CharacterMovement`)))

(fn `StopSprint`
  (set `CharacterMovementComponent.MaxWalkSpeed` (`self.WalkSpeed`) (`self.CharacterMovement`)))

(fn `UpdatePlayerState`
  (if (`self.bHasBall`)
    (set `self.State_BP` "NewEnumerator0")
    (else
      (set `self.State_BP` "NewEnumerator6"))))

(fn `UserConstructionScript`)