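; BP_AICharacter is an AI-named character for a ball game, storing the first player's character as its defense target on BeginPlay.
; Sprint and StopSprint switch the movement component's max walk speed between the sprint and walk values.
; UpdatePlayerState sets an enum state according to whether the character has the ball.
; The Blueprint has no active Tick or overlap logic and calls none of these functions itself.
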(event `self.ReceiveBeginPlay`
  (set `self.DefenseTarget` (`GameplayStatics.GetPlayerCharacter` 0)))

(fn `Sprint`
  (set `CharacterMovementComponent.MaxWalkSpeed` (`self.SprintSpeed`) (`self.CharacterMovement`)))

(fn `StopSprint`
  (set `CharacterMovementComponent.MaxWalkSpeed` (`self.WalkSpeed`) (`self.CharacterMovement`)))

(fn `UpdatePlayerState`
  (if (`self.bHasBall`)
    (set `self.State_BP` "NewEnumerator0")
    (else
      (set `self.State_BP` "NewEnumerator6"))))

(fn `UserConstructionScript`)