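; Basketball actor that is held, dribbled and launched at a target by its owner character.
; Tick drives a ball state: snap to the hand socket, or lerp down and up with a curve arc, offset by move input.
; LaunchToTarget solves ballistic velocity from flight time and gravity, then detaches and enables physics.
; Overlapping the owner attaches it; hits play rate-limited audio with impulse-scaled volume and pitch.
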(event `self.Ball.OnComponentHit`
  (params (HitComponent :type "PrimitiveComponent Object Reference") (OtherActor :type "Actor Object Reference") (OtherComp :type "PrimitiveComponent Object Reference") (NormalImpulse :type "Vector Structure") (Hit :type "HitResult Structure (by ref)"))
  (bind _returnvalue (`KismetMathLibrary.VSize` NormalImpulse))
  (bind _ball_hit_sound (`self.Ball_hit_Sound`))
  (if (`KismetMathLibrary.InRange_FloatFloat` _returnvalue 50.0 10000.0)
    (`/Engine/EditorBlueprintResources/StandardMacros.DoOnce` false :!label _label
      (:`Completed`
        (`AudioComponent.SetVolumeMultiplier` _ball_hit_sound (`KismetMathLibrary.MapRangeClamped` _returnvalue 0.0 2500.0 0.0 1.0))
        (`AudioComponent.SetFloatParameter` _ball_hit_sound "pitch" (`KismetMathLibrary.MapRangeClamped` _returnvalue 20.0 1000.0 0.85 1.2))
        (`AudioComponent.Play` _ball_hit_sound 0.0)
        (`KismetSystemLibrary.Delay` 0.2)
        (goto _label :!via `Reset`)))))

(event `self.ReceiveTick`
  (params (DeltaSeconds :type "Float (single-precision)"))
  (switch `/Game/Blueprint/EBallState` (`self.BallState`)
    (:`NewEnumerator0`
      (`self.SnapToHand`))
    (:`NewEnumerator1`
      (bind _output_get (set `self.MoveAlpha` (`KismetMathLibrary.FClamp` (+ (`self.MoveAlpha`) (* DeltaSeconds (`self.MoveSpeed`)))) :!label _label_2))
      (bind (_returnvalue_x _returnvalue_y _returnvalue_z) (`KismetMathLibrary.BreakVector` (`KismetMathLibrary.VLerp` (`self.CurrentStartLocation`) (`self.CurrentTargetLocation`) _output_get)))
      (`self.K2_SetActorLocation` (+ (0.0 0.0 0.0) (`KismetMathLibrary.MakeVector` _returnvalue_x _returnvalue_y (+ (* (`CurveFloat.GetFloatValue` (`self.BallArcCurve`) (`self.MoveAlpha`)) (`self.ArcHeight`)) _returnvalue_z))))
      (if (>= (`self.MoveAlpha`) 1.0)
        (switch `/Game/Blueprint/EBallState` "NewEnumerator0"
          (:`NewEnumerator2`
            (`self.SetAttached`)))))
    (:`NewEnumerator2`
      (goto _label_2))))

(event `self.ReceiveBeginPlay`)

(event `self.ReceiveActorBeginOverlap`
  (params (OtherActor :type "Actor Object Reference"))
  (if (== OtherActor (`self.OwnerCharacter`))
    (set `/Game/Blueprint/Character/BP_CharacterBase.MainState` "NewEnumerator2" (`self.OwnerCharacter`))
    (bind _returnvalue (`self.K2_AttachToComponent` (`Character.Mesh` (`self.OwnerCharacter`)) (`self.CurrentHandSocketName`) "SnapToTarget" "SnapToTarget" "SnapToTarget"))
    (if _returnvalue
      _)))

(fn `LaunchToTarget`
  (params (InTargetLocation :type "Vector Structure"))
  (locals (NewLocalVar :type "Vector Structure" :default (0.0 0.0 0.0)))
  (bind _sphere (`self.Sphere`))
  (bind _flighttime (`self.FlightTime`))
  (bind (_returnvalue_x _returnvalue_y _returnvalue_z) (`KismetMathLibrary.BreakVector` (- (- InTargetLocation (`self.K2_GetActorLocation`)) (* (* (* (`self.FlightTime`) (`self.FlightTime`)) (`KismetMathLibrary.MakeVector` 0.0 0.0 (`self.GravityZ`))) 0.5))))
  (bind _output_get (set `self.LaunchVelocity` (`KismetMathLibrary.MakeVector` (/ _returnvalue_x _flighttime) (/ _returnvalue_y _flighttime) (/ _returnvalue_z _flighttime))))
  (`self.K2_DetachFromActor` "KeepWorld" "KeepWorld" "KeepWorld")
  (set `self.BallState` "NewEnumerator3")
  (`PrimitiveComponent.SetSimulatePhysics` _sphere true)
  (`PrimitiveComponent.SetEnableGravity` _sphere true)
  (`PrimitiveComponent.SetPhysicsLinearVelocity` _sphere _output_get false "None"))

(fn `SetAttached`
  (set `self.BallState` "NewEnumerator0")
  (`self.SnapToHand`))

(fn `SetOwnerCharacter`
  (params (NewOwnerCharacter :type "/Game/Blueprint/Character/BP_CharacterBase Object Reference"))
  (set `self.OwnerCharacter` NewOwnerCharacter))

(fn `SnapToHand`
  (bind _ownercharacter (`self.OwnerCharacter`))
  ; 공을 손위치로 보내는 함수
  (`/Engine/EditorBlueprintResources/StandardMacros.IsValid` (`self.OwnerCharacter`)
    (:`Is Valid`
      (`self.K2_SetActorLocation` (`SceneComponent.GetSocketLocation` (`Character.Mesh` _ownercharacter) (`/Game/Blueprint/Character/BP_CharacterBase.SocketName` _ownercharacter))))))

(fn `StartMoveDown`
  (bind (_returnvalue_x _returnvalue_y _returnvalue_z) (`KismetMathLibrary.BreakVector` (`self.K2_GetActorLocation`)))
  (bind _ownercharacter (`self.OwnerCharacter`))
  (bind (_returnvalue_x_2 _returnvalue_y_2) (`KismetMathLibrary.BreakVector` (`SceneComponent.GetSocketLocation` (`Character.Mesh` (`self.OwnerCharacter`)) (`self.CurrentHandSocketName`))))
  (set `self.BallState` "NewEnumerator1")
  (set `self.CurrentStartLocation` (`KismetMathLibrary.MakeVector` _returnvalue_x _returnvalue_y _returnvalue_z))
  (set `self.CurrentTargetLocation` (`KismetMathLibrary.MakeVector` (+ _returnvalue_x_2 (* (`/Game/Blueprint/Character/BP_CharacterBase.MoveInputX` _ownercharacter) 70.0)) (+ _returnvalue_y_2 (* (`/Game/Blueprint/Character/BP_CharacterBase.MoveInputY` _ownercharacter) 70.0)) 12.0))
  (set `self.MoveAlpha` 0.0)
  (set `self.Zvalue` _returnvalue_z))

(fn `StartMoveUp`
  (bind _ownercharacter (`self.OwnerCharacter`))
  (bind (_returnvalue_x _returnvalue_y) (`KismetMathLibrary.BreakVector` (`SceneComponent.GetSocketLocation` (`Character.Mesh` (`self.OwnerCharacter`)) (`self.CurrentHandSocketName`))))
  (set `self.BallState` "NewEnumerator2")
  (set `self.CurrentStartLocation` (`self.K2_GetActorLocation`))
  (set `self.CurrentTargetLocation` (`KismetMathLibrary.MakeVector` (+ _returnvalue_x (* (`/Game/Blueprint/Character/BP_CharacterBase.MoveInputX` _ownercharacter) 70.0)) (+ _returnvalue_y (* (`/Game/Blueprint/Character/BP_CharacterBase.MoveInputY` _ownercharacter) 70.0)) (`self.Zvalue`)))
  (set `self.MoveAlpha` 0.0))

(fn `UserConstructionScript`)