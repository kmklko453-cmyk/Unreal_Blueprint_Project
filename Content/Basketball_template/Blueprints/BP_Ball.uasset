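; BP_Ball is a basketball actor that dribbles between its owner character's hand and the ground, with impact sounds.
; Once MoveToHand or MoveToGround starts movement, Tick lerps the ball to the target and flips direction on arrival.
; Targets are snapshotted from the hand socket at each leg's start, with ground being a fixed offset below it.
; Hit events scale sound volume and pitch by impulse strength, throttled by a resetting DoOnce.
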(event `self.Ball.OnComponentHit`
  (params (HitComponent :type "PrimitiveComponent Object Reference") (OtherActor :type "Actor Object Reference") (OtherComp :type "PrimitiveComponent Object Reference") (NormalImpulse :type "Vector Structure") (Hit :type "HitResult Structure (by ref)"))
  (bind _returnvalue (`KismetMathLibrary.VSize` NormalImpulse))
  (bind _ball_hit_sound (`self.Ball_hit_Sound`))
  (if (`KismetMathLibrary.InRange_FloatFloat` _returnvalue 50.0 10000.0)
    (`/Engine/EditorBlueprintResources/StandardMacros.DoOnce` false :!label _label
      (:`Completed`
        (`AudioComponent.SetVolumeMultiplier` _ball_hit_sound (`KismetMathLibrary.MapRangeClamped` _returnvalue 0.0 2500.0 0.0 1.0))
        (`AudioComponent.SetFloatParameter` _ball_hit_sound "pitch" (`KismetMathLibrary.MapRangeClamped` _returnvalue 20.0 1000.0 0.85 1.2))
        (`AudioComponent.Play` _ball_hit_sound 0.0)
        (`KismetSystemLibrary.Delay` 0.2)
        (goto _label :!via `Reset`)))))

(event `self.ReceiveTick`
  (params (DeltaSeconds :type "Float (single-precision)"))
  ; 공 이동 로직
  (if (`self.bIsMoving`)
    (bind _output_get (set `self.DribbleAlpha` (+ (* DeltaSeconds (`self.DribbleSpeed`)) (`self.DribbleAlpha`))))
    (`self.K2_SetActorLocation` (`KismetMathLibrary.VLerp` (`self.StartLocation`) (`self.TargetLocation`) _output_get))
    (if (>= (`self.DribbleAlpha`) 1.0)
      (`self.K2_SetActorLocation` (`self.TargetLocation`))
      (if (`self.bMoveToHand`)
        (`self.MoveToGround`)
        (else
          (`self.MoveToHand`))))))

(fn `MoveToGround`
  (set `self.StartLocation` (`self.K2_GetActorLocation`))
  (`/Engine/EditorBlueprintResources/StandardMacros.IsValid` (`self.OwnerCharacter`)
    (:`Is Valid`
      (set `self.TargetLocation` (`KismetMathLibrary.MakeVector` (.x (`SceneComponent.GetSocketLocation` (`Character.Mesh` (`self.OwnerCharacter`)) (`self.HandSocketName`))) (.y (`SceneComponent.GetSocketLocation` (`Character.Mesh` (`self.OwnerCharacter`)) (`self.HandSocketName`))) (- (.z (`SceneComponent.GetSocketLocation` (`Character.Mesh` (`self.OwnerCharacter`)) (`self.HandSocketName`))) (`self.GroundOffset`))))
      (set `self.DribbleAlpha` 0.0)
      (set `self.bMoveToHand` false)
      (set `self.bIsMoving` true))))

(fn `MoveToHand`
  (set `self.StartLocation` (`self.K2_GetActorLocation` self))
  (`/Engine/EditorBlueprintResources/StandardMacros.IsValid` (`self.OwnerCharacter`)
    (:`Is Valid`
      (set `self.TargetLocation` (`SceneComponent.GetSocketLocation` (`Character.Mesh` (`self.OwnerCharacter`)) (`self.HandSocketName`)))
      (set `self.DribbleAlpha` 0.0)
      (set `self.bMoveToHand` true)
      (set `self.bIsMoving` true))))

(fn `SetOwnerCharacter`
  (params (NewOwnerCharacter :type "/Game/Blueprint/BP_Character Object Reference"))
  (set `self.OwnerCharacter` NewOwnerCharacter))

(fn `UserConstructionScript`)